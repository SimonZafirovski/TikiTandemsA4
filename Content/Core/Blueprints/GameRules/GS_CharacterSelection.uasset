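; Game state for the character selection level, coordinating arena choice and the move into the match.
; MC_SetArena flip-flops day and night, swapping tagged sky actors, fading directional light through a timeline and saving the arena type to the game instance.
; Menu and start events call GetAllPlayerControllers, which returns only the game mode's first controller.
; ArenaChosen triggers face-off animations, binding each selection actor's event to show every player's loading screen.
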(event Custom|MC_SetArena
  ;[1 1 1] SwitchArena types logic
  (bind _returnvalue (Actor|GetActorOfClass "/Script/Engine.DirectionalLight"))
  (bind _asgi_tiki_tandems (Utilities|Casting|CastToGI_TikiTandems (Game|GetGameInstance)))
  (Utilities|FlowControl|FlipFlop
    (:A
      (Utilities|SetNightArena)
      (Variables|/Game/Core/Blueprints/GameRules/GI_TikiTandems.GI_TikiTandems_C|SeteArenaType _asgi_tiki_tandems "NewEnumerator1")
      (bind _shiftdaynight (Timeline|ShiftTimeOfDay Play)
        (:Update
          (Utilities|IsValid (Variables|/Script/Engine.Light|GetLightComponent _returnvalue)
            (:Is%20Valid
              (Rendering|Components|Light|SetIntensity (Variables|/Script/Engine.Light|GetLightComponent _returnvalue) _shiftdaynight))))))
    (:B
      (Utilities|SetDayArena)
      (Variables|/Game/Core/Blueprints/GameRules/GI_TikiTandems.GI_TikiTandems_C|SeteArenaType _asgi_tiki_tandems "NewEnumerator0")
      (Timeline|ShiftTimeOfDay Reverse))))

(event Custom|OpenArenaLogic
  ;[1 1 1] Character selection logic
  (bind _asbpc_character_selection (Utilities|GetAllPlayerControllers))
  (Default|StartGame _asbpc_character_selection))

(event Custom|OpenArenaSelectionMenu
  ;[1 1 1] Character selection logic
  (bind _asbpc_character_selection (Utilities|GetAllPlayerControllers))
  (Default|ChooseArena _asbpc_character_selection))

(event Custom|ArenaChosen
  ;[1 1 1] Show loading screens for level travel logic
  (bind _outactors (Actor|GetAllActorsOfClass "/Game/Core/Blueprints/Characters/CharacterSelector/BP_CharacterSelection.BP_CharacterSelection_C"))
  (for _array_element _outactors
    (Default|FaceOffAnimation _array_element)
    (EventDispatchers|BindEventtoShowLoadingScreen _array_element (delegate Custom|ShowLoadingScreens))))

(event Custom|ShowLoadingScreens
  ;[1 1 1] Show loading screens for level travel logic
  (for _array_element (Variables|Default|GetPlayerArray)
    (bind _asbpc_character_selection (Utilities|Casting|CastToBPC_CharacterSelection (Game|GetPlayerController _array_element)))
    (Default|ShowLoadingScreen _asbpc_character_selection)))

(fn ConstructionScript)