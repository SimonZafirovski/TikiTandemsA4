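; Game mode for the two-player character selection lobby, assigning joining controllers as P1 or P2 by login order.
; Join functions set names, waiting-widget visibility, default character and player index; P1 gets exit-only input until P2 arrives and both receive input.
; P2 logout restores the waiting state and strips P1's input.
; Other events open arena choice on P2's controller or destroy the session behind a loading screen; LaunchArena is empty.
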(event Custom|MC_SetP1Name
  (params (P1Name :type Text))
  ;[1 1 1] PlayerData setup
  (Variables|Default|SetP1Name P1Name))

(event Custom|MC_SetP2Widgets
  (params (IsWaitingVisible? :type ESlateVisibility%20Enum :default "Visible"))
  ;[1 1 1] PlayerData setup
  (Variables|Default|SetIsWaitingVisible? IsWaitingVisible?))

(event Custom|MC_SetDefaultCharacter
  (params (PlayerController :type Player%20Controller%20Object%20Reference))
  ;[1 1 1] PlayerData setup
  (bind _asbp_character_selection (Utilities|Casting|CastToBP_CharacterSelection (Pawn|GetControlledPawn PlayerController)))
  (Variables|/Game/Core/Blueprints/Characters/CharacterSelector/BP_CharacterSelection.BP_CharacterSelection_C|SeteCurrentCharacter _asbp_character_selection "NewEnumerator0"))

(event Custom|MC_SetP2Name
  (params (P2Name :type Text))
  ;[1 1 1] PlayerData setup
  (Variables|Default|SetP2Name P2Name))

(event Custom|MC_SetArenaWidget
  ;[1 1 1] Activate arena switching widget logic
  (bind _asbpc_character_selection (Utilities|Casting|CastToBPC_CharacterSelection (Utilities|Array|Get(acopy) (Variables|Default|GetPlayerControllers) 1)))
  (Default|ChooseArena _asbpc_character_selection))

(event Custom|CloseTheGame
  (params (PlayerController :type Player%20Controller%20Object%20Reference))
  ;[1 1 1] Leaving match loading screen
  (|DestroySession PlayerController
    (:then
      (bind _asgi_tiki_tandems (Utilities|Casting|CastToGI_TikiTandems (Game|GetGameInstance)))
      (Default|ShowLoadingScreen _asgi_tiki_tandems))))

(event EventPostLogin
  (params (NewPlayer :type Player%20Controller%20Object%20Reference))
  ;[1 1 1] Lobby setup logic
  (|CallParentFunction NewPlayer)
  (bind _returnvalue (Utilities|Array|Add (Variables|Default|GetPlayerControllers) NewPlayer))
  (if (== _returnvalue 0)
    (CallFunction|P1JoinedGame "Player1" NewPlayer)
    (else
      (CallFunction|P2JoinedGame "Player2" NewPlayer))))

(event EventOnLogout
  (params (ExitingController :type Controller%20Object%20Reference))
  ;[1 1 1] P2 leaving the game logic
  (bind _asplayer_controller (Utilities|Casting|CastToPlayerController ExitingController))
  (if (== _asplayer_controller (Utilities|Array|Get(acopy) (Variables|Default|GetPlayerControllers) 1))
    (CallFunction|P2LeftGame)))

(fn ConstructionScript)

(fn LaunchArena)

(fn P1JoinedGame
  (params (P1Name :type Text) (NewPlayerController :type Player%20Controller%20Object%20Reference))
  (bind _output_get (Variables|Default|SetP1Name P1Name))
  (CallFunction|MCSetP1Name _output_get)
  (CallFunction|MCSetP2Widgets "Visible")
  (bind _asbpc_character_selection (Utilities|Casting|CastToBPC_CharacterSelection NewPlayerController))
  (Default|LobbySetup _asbpc_character_selection)
  (CallFunction|MCSetDefaultCharacter _asbpc_character_selection)
  (CallFunction|RemoveAllInputMappingContexts _asbpc_character_selection)
  (CallFunction|AddInputMappingContext _asbpc_character_selection "/Game/Core/Blueprints/Input/InputActionMappings/IMC_Exit.IMC_Exit" 1)
  (Variables|/Game/Core/Blueprints/Input/Controllers/BPC_CharacterSelection.BPC_CharacterSelection_C|SetPlayerIndex _asbpc_character_selection 0))

(fn P2JoinedGame
  (params (P2Name :type Text) (NewPlayerController :type Player%20Controller%20Object%20Reference))
  (bind _output_get (Variables|Default|SetP2Name P2Name))
  (CallFunction|MCSetP2Name _output_get)
  (bind _output_get_2 (Variables|Default|SetIsWaitingVisible? "Hidden"))
  (CallFunction|MCSetP2Widgets _output_get_2)
  (bind _asbpc_character_selection (Utilities|Casting|CastToBPC_CharacterSelection NewPlayerController))
  (Default|LobbySetup _asbpc_character_selection)
  (CallFunction|MCSetDefaultCharacter _asbpc_character_selection)
  (Variables|/Game/Core/Blueprints/Input/Controllers/BPC_CharacterSelection.BPC_CharacterSelection_C|SetPlayerIndex _asbpc_character_selection 1)
  (for _array_element (Variables|Default|GetPlayerControllers)
    (Default|AddInputtoOwningPlayer (.AsBPC%20Character%20Selection (Utilities|Casting|CastToBPC_CharacterSelection _array_element)))
    (Default|CLEnableP2 (.AsBPC%20Character%20Selection (Utilities|Casting|CastToBPC_CharacterSelection _array_element)))))

(fn OnRepP2Name
  (for _array_element (Variables|Default|GetPlayerControllers)
    (bind _asbpc_character_selection (Utilities|Casting|CastToBPC_CharacterSelection _array_element))
    (Utilities|FlowControl|Sequence
      (:then_0
        (Variables|/Game/Core/Blueprints/Input/Controllers/BPC_CharacterSelection.BPC_CharacterSelection_C|SetP1Name _asbpc_character_selection (Variables|Default|GetP1Name)))
      (:then_1
        (Variables|/Game/Core/Blueprints/Input/Controllers/BPC_CharacterSelection.BPC_CharacterSelection_C|SetP2Name _asbpc_character_selection (Variables|Default|GetP2Name))))))

(fn P2LeftGame
  (bind _playercontrollers (Variables|Default|GetPlayerControllers))
  (bind _output (Utilities|Array|Get(acopy) _playercontrollers))
  (Variables|Default|SetIsP2Visible? "Hidden")
  (CallFunction|MCSetP2Widgets "Visible")
  (Utilities|IsValid _output
    (:Is%20Valid
      (bind _asbpc_character_selection (Utilities|Casting|CastToBPC_CharacterSelection _output))
      (Default|CLDisableP2 _asbpc_character_selection)
      (CallFunction|RemoveAllInputMappingContexts _asbpc_character_selection))))