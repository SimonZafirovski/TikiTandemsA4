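; Game State for the Tiki arena match, running the countdown timer, totem progress tracking and match flow.
; BeginPlay finds the totem, starts the timer, game mode and quicksand; Tick mirrors wing and fist yaw as win and power-up progress.
; Events end the cinematic once two players are ready, then set up controls and team overlays by server flag.
; A lone remaining player triggers slow-motion match end; timer expiry quits the game.
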(event Custom|MC_StartGameTimer
  ;[1 1 1] Timer logic
  (Utilities|Time|SetTimerbyEvent (delegate Custom|UpdateGameTimer) 1.0 true))

(event Custom|UpdateGameTimer
  ;[1 1 1] Timer logic
  (if (== (Variables|Default|GetSeconds) 0)
    (if (== (Variables|Default|GetMinutes) 0)
      (Game|QuitGame 0 "Quit" false)
      (else
        (bind _result (Math|Integer|DecrementInt (Variables|Default|GetMinutes))
          (:%20%20
            (Variables|Default|SetMinutes _result)
            (Variables|Default|SetSeconds 59)))))
    (else
      (bind _result_2 (Math|Integer|DecrementInt (Variables|Default|GetSeconds))
        (:%20%20
          (Variables|Default|SetSeconds _result_2))))))

(event Custom|CheckIfAllPlayersAreReady
  ;[1 1 1] Check if all players are ready to end animation logic
  (for _array_element (Variables|Default|GetPlayerArray)
    (bind _asps_tiki_arena (Utilities|Casting|CastToPS_TikiArena _array_element))
    (if (Variables|/Game/Core/Blueprints/GameRules/PS_TikiArena.PS_TikiArena_C|GetbReady? _asps_tiki_arena)
      (Math|Integer|IncrementInt (Variables|Default|GetiCounter))))
  (if (>= (Variables|Default|GetiCounter) 2)
    (bind _asgm_arena (Utilities|Casting|CastToGM_Arena (Game|GetGameMode)))
    (for _array_element_2 (Variables|/Game/Core/Blueprints/GameRules/GameModes/GM_Arena.GM_Arena_C|GetPlayerControllers _asgm_arena)
      (bind _asbpc_tiki_arena (Utilities|Casting|CastToBPC_TikiArena _array_element_2))
      (Default|CallEndCinematic _asbpc_tiki_arena))))

(event Custom|MC_AddControls
  ;[1 1 1] Add input to each player logic
  (for _array_element (Variables|Default|GetPlayerArray)
    (bind _asbpc_tiki_arena (Utilities|Casting|CastToBPC_TikiArena (Game|GetPlayerController _array_element)))
    (Default|AddControls _asbpc_tiki_arena)
    (if (Variables|/Game/Core/Blueprints/Input/Controllers/BPC_TikiArena.BPC_TikiArena_C|GetbIsServer? _asbpc_tiki_arena)
      (Pawn|SetControlRotation _asbpc_tiki_arena (Math|Rotator|MakeRotator 0.0 5.0 9e+01))
      (else
        (Pawn|SetControlRotation _asbpc_tiki_arena (Math|Rotator|MakeRotator 0.0 5.0 -9e+01)))))
  (CallFunction|MCStartGameTimer)
  (CallFunction|SetTotemObjects)
  (CallFunction|CLSetTeamOverlay))

(event Custom|CL_SetTeamOverlay
  ;[1 1 1] Set player team colors/overlay logic
  (Utilities|FlowControl|Delay 0.2)
  (for _array_element (Variables|Default|GetPlayerArray)
    (bind _asbpc_tiki_arena (Utilities|Casting|CastToBPC_TikiArena (Game|GetPlayerController _array_element)))
    (bind _asbp_tiki (Utilities|Casting|CastToBP_Tiki (Pawn|GetControlledPawn _asbpc_tiki_arena)))
    (Default|SRSetTeamOverlayColor _asbp_tiki (Variables|/Game/Core/Blueprints/Input/Controllers/BPC_TikiArena.BPC_TikiArena_C|GetbIsServer? _asbpc_tiki_arena))))

(event Custom|MC_EndMatch
  (params (WhoWon? :type Boolean))
  ;[1 1 1] MatchEnd/Who won logic
  (Viewport|RemoveAllWidgets)
  (Utilities|Time|SetGlobalTimeDilation 0.2)
  (Utilities|Casting|CastToGI_TikiTandems (Game|GetGameInstance))
  (if WhoWon?
    _))

(event EventTick
  (params (DeltaSeconds :type Float%20%28single-precision%29))
  (bind _playerarray (Variables|Default|GetPlayerArray))
  (bind _totem (Variables|Default|GetTotem))
  ;[1 1 1] Check status of totem elements
  (Variables|Default|SetWinProgress (.yaw (Variables|/Script/Engine.SceneComponent|GetRelativeRotation (Variables|/Game/Core/Blueprints/WinCondition/BP_WinCon.BP_WinCon_C|GetWingsBase _totem))))
  (Variables|Default|SetPowerUpProgress (.yaw (Variables|/Script/Engine.SceneComponent|GetRelativeRotation (Variables|/Game/Core/Blueprints/WinCondition/BP_WinCon.BP_WinCon_C|GetFistsBase _totem))))
  (if (Variables|Default|GetbMatchHasStarted)
    (if (<= (Utilities|Array|Length _playerarray) 1)
      (Utilities|FlowControl|DoOnce false
        (:Completed
          (for _array_element _playerarray
            (bind _asps_tiki_arena (Utilities|Casting|CastToPS_TikiArena _array_element))
            (CallFunction|MCEndMatch (Variables|/Game/Core/Blueprints/GameRules/PS_TikiArena.PS_TikiArena_C|GetbIsServer? _asps_tiki_arena))))))))

(event EventBeginPlay
  ;[1 1 1] BeginPlay logic
  (bind _returnvalue (Actor|GetActorOfClass "/Game/Core/Blueprints/WinCondition/BP_WinCon.BP_WinCon_C"))
  (Variables|Default|SetTotem _returnvalue)
  (CallFunction|MCStartGameTimer)
  (Variables|Default|SetbMatchHasStarted true)
  (bind _asgm_arena (Utilities|Casting|CastToGM_Arena (Game|GetGameMode)))
  (Default|CallStartGame _asgm_arena)
  (bind _outactors (Actor|GetAllActorsOfClass "/Game/Core/Blueprints/Obstacles/BP_Quicksand.BP_Quicksand_C"))
  (for _array_element _outactors
    (Class|BPISync|BISQuicksandStart(Message) _array_element)))

(fn ConstructionScript)

(fn SetTotemObjects
  (bind _returnvalue (Actor|GetActorOfClass "/Game/Core/Blueprints/WinCondition/BP_WinCon.BP_WinCon_C"))
  (Variables|Default|SetWinCondition (Variables|/Game/Core/Blueprints/WinCondition/BP_WinCon.BP_WinCon_C|GetWingsBase _returnvalue))
  (Variables|Default|SetPowerUpCondition (Variables|/Game/Core/Blueprints/WinCondition/BP_WinCon.BP_WinCon_C|GetFistsBase _returnvalue)))