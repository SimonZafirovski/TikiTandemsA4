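; Player controller for the two-player online lobby, handling character selection, locking and arena choice.
; Enhanced Input cycles and locks each player's selector actor, with client actions relayed through server-to-multicast events.
; Replicated lock flags swap input mapping contexts, the selected character sets the GameInstance player class, and both locks hand off to GameState arena logic.
; When the host exits with P2 present, the client starts a new server.
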(event Custom|CL_SetPlayerClass
  ;[1 1 1] Set player class in GI logic
  (bind _characterclass (CallFunction|GetPlayerCharacterClass (Variables|Default|GeteSelectedCharacter)))
  (bind _asgi_tiki_tandems (Utilities|Casting|CastToGI_TikiTandems (Game|GetGameInstance)))
  (Variables|/Game/Core/Blueprints/GameRules/GI_TikiTandems.GI_TikiTandems_C|SetPlayerClass _asgi_tiki_tandems _characterclass))

(event Custom|CL_EnableP2
  (bind _characterselectionref (Variables|Default|GetCharacterSelectionRef))
  ;[1 1 1] ShowP2 On joining
  (Rendering|SetActorHiddenInGame (Variables|Default|GetP2Actor) false)
  (Widget|SetVisibility (Variables|/Game/Core/Widgets/CharacterSelection/W_CharacterSelectionScreen.W_CharacterSelectionScreen_C|GetWaiting _characterselectionref) "Hidden")
  (Widget|SetVisibility (Variables|/Game/Core/Widgets/CharacterSelection/W_CharacterSelectionScreen.W_CharacterSelectionScreen_C|GetW_P2Name _characterselectionref) "Visible"))

(event Custom|MC_LockCharacter
  (params (Target :type BP%20Character%20Selection%20Object%20Reference) (WorldButton :type W%20World%20Button%20Object%20Reference))
  ;[1 1 1] Lock character and arena logic
  (Default|LockCharacter Target WorldButton)
  (if (Variables|/Game/Core/Blueprints/Characters/CharacterSelector/BP_CharacterSelection.BP_CharacterSelection_C|GetbCanLock? Target)
    (Utilities|FlowControl|FlipFlop
      (:A
        (Variables|Default|SetP2Locked? true)
        (Utilities|FlowControl|Delay 0.01)
        (if (Utilities|AreBothPlayersReady?)
          (Default|OpenArenaSelectionMenu (Variables|Default|GetGSCharacterSelectionRef))))
      (:B
        (Variables|Default|SetP2Locked? false)))))

(event Custom|SR_LockCharacter
  (params (Target :type BP%20Character%20Selection%20Object%20Reference) (WorldButton :type W%20World%20Button%20Object%20Reference))
  ;[1 1 1] Lock character and arena logic
  (CallFunction|MCLockCharacter Target WorldButton))

(event Custom|StartGame
  ;[1 1 1] Start the game logic
  (Default|LockArena (Variables|Default|GetCharacterSelectionRef))
  (Default|ArenaChosen (Variables|Default|GetGSCharacterSelectionRef)))

(event Custom|CL_DisableP2
  (bind _characterselectionref (Variables|Default|GetCharacterSelectionRef))
  ;[1 1 1] ShowP2 On joining
  (Rendering|SetActorHiddenInGame (Variables|Default|GetP2Actor) true)
  (Widget|SetVisibility (Variables|/Game/Core/Widgets/CharacterSelection/W_CharacterSelectionScreen.W_CharacterSelectionScreen_C|GetWaiting _characterselectionref) "Visible")
  (Widget|SetVisibility (Variables|/Game/Core/Widgets/CharacterSelection/W_CharacterSelectionScreen.W_CharacterSelectionScreen_C|GetW_P2Name _characterselectionref) "Hidden"))

(event Custom|LeaveGame
  ;[1 1 1] Server leaving and Client creating new match as Server logic
  (Utilities|Time|ClearandInvalidateTimerbyHandle (stale Input|EnhancedActionEvents|EnhancedInputActionIA_Exit _returnvalue))
  (Game|OpenLevel(byObjectReference) "/Game/maps/L_MainMenu.L_MainMenu"))

(event Custom|StartNewServer
  ;[1 1 1] Server leaving and Client creating new match as Server logic
  (CallFunction|CLLoadingScreen)
  (bind _asgi_tiki_tandems (Utilities|Casting|CastToGI_TikiTandems (Game|GetGameInstance)))
  (Utilities|FlowControl|Delay 1.0)
  (Default|StartNewServer _asgi_tiki_tandems))

(event Custom|CL_AddInputToOwningPlayer
  ;[1 1 1] Add input
  (CallFunction|AddInputMappingContext self "/Game/Core/Blueprints/Input/InputActionMappings/IMC_CharacterSelection.IMC_CharacterSelection" 1))

(event Custom|CL_LoadingScreen
  ;[1 1 1] Show loading screen
  (bind _loadingscreenwidget (CallFunction|CreateLoadingScreen self))
  (bind _output_get (Variables|Default|SetwLoadingScreen _loadingscreenwidget))
  (Utilities|FlowControl|Delay 1.0)
  (Widget|RemovefromParent _output_get))

(event Custom|CL_LobbySetup
  (params (PlayerIndex :type Integer))
  ;[1 1 1] Lobby setup logic
  (Input|SetInputModeGameOnly self false)
  (CallFunction|CLCreateWidgets)
  (CallFunction|SetSelectedPlayer PlayerIndex))

(event Custom|MC_SwitchCharacter
  (params (NextPrev :type Boolean) (WhichPlayer? :type BP%20Character%20Selection%20Object%20Reference))
  ;[1 1 1] Character and map switching logic
  (CallFunction|SwitchCharacter NextPrev WhichPlayer?))

(event Custom|SR_SwitchCharacter
  (params (NextPrev :type Boolean) (WhichPlayer? :type BP%20Character%20Selection%20Object%20Reference))
  ;[1 1 1] Character and map switching logic
  (CallFunction|MCSwitchCharacter NextPrev WhichPlayer?))

(event Custom|ChooseArena
  (bind _self self)
  ;[1 1 1] Set arena widget logic
  (Default|ChooseArena (Variables|Default|GetCharacterSelectionRef))
  (if (Utilities|IsServer?)
    (CallFunction|AddInputMappingContext _self "/Game/Core/Blueprints/Input/InputActionMappings/IMC_CharacterSelection.IMC_CharacterSelection" 1)
    (CallFunction|RemoveInputMappingContext _self "/Game/Core/Blueprints/Input/InputActionMappings/IMC_Lock.IMC_Lock")
    (bind _asgm_character_selection (Utilities|Casting|CastToGM_CharacterSelection (Game|GetGameMode)))
    (Default|MCSetArenaWidget _asgm_character_selection)
    (else
      (CallFunction|RemoveAllInputMappingContexts _self)
      (CallFunction|SRSetArenaWidget))))

(event Custom|CL_CreateWidgets
  ;[1 1 1] Create widgets logic
  (bind _returnvalue (UserInterface|CreateWidget "/Game/Core/Widgets/CharacterSelection/W_CharacterSelectionScreen.W_CharacterSelectionScreen_C" self))
  (bind _output_get (Variables|Default|SetCharacterSelectionRef _returnvalue))
  (UserInterface|Viewport|AddtoViewport _output_get 0)
  (if (not (Utilities|IsServer?))
    (Variables|/Script/UMG.Widget|SetVisibility (Variables|/Game/Core/Widgets/CharacterSelection/W_CharacterSelectionScreen.W_CharacterSelectionScreen_C|GetWaiting (Variables|Default|GetCharacterSelectionRef)) "Hidden")))

(event Custom|SR_SetArenaWidget
  ;[1 1 1] Set arena widget logic
  (bind _asgm_character_selection (Utilities|Casting|CastToGM_CharacterSelection (Game|GetGameMode)))
  (Default|MCSetArenaWidget _asgm_character_selection))

(event Input|EnhancedActionEvents|EnhancedInputActionIA_NextSelection
  (params (ActionValue :type Boolean) (ElapsedSeconds :type Float%20%28double-precision%29) (TriggeredSeconds :type Float%20%28double-precision%29) (InputAction :type Input%20Action%20Object%20Reference :default "/Game/Core/Blueprints/Input/InputActions/IA_NextSelection.IA_NextSelection"))
  (bind _playeractor (Variables|Default|GetPlayerActor))
  ;[1 1 1] Character and map switching logic
  (:Started
    (Variables|Default|SetbNextPrevious true)
    (if (Utilities|AreBothPlayersReady?)
      (Default|MCSetArena (Variables|Default|GetGSCharacterSelectionRef))
      (elif (Utilities|IsServer?)
        (CallFunction|SwitchCharacter (Variables|Default|GetbNextPrevious) _playeractor)
        (else
          (CallFunction|SRSwitchCharacter (Variables|Default|GetbNextPrevious) _playeractor))))))

(event Input|EnhancedActionEvents|EnhancedInputActionIA_PreviousSelection
  (params (ActionValue :type Boolean) (ElapsedSeconds :type Float%20%28double-precision%29) (TriggeredSeconds :type Float%20%28double-precision%29) (InputAction :type Input%20Action%20Object%20Reference :default "/Game/Core/Blueprints/Input/InputActions/IA_PreviousSelection.IA_PreviousSelection"))
  (bind _playeractor (Variables|Default|GetPlayerActor))
  ;[1 1 1] Character and map switching logic
  (:Started
    (Variables|Default|SetbNextPrevious false)
    (if (Utilities|AreBothPlayersReady?)
      (Default|MCSetArena (Variables|Default|GetGSCharacterSelectionRef))
      (elif (Utilities|IsServer?)
        (CallFunction|SwitchCharacter (Variables|Default|GetbNextPrevious) _playeractor)
        (else
          (CallFunction|SRSwitchCharacter (Variables|Default|GetbNextPrevious) _playeractor))))))

(event Input|EnhancedActionEvents|EnhancedInputActionIA_Next
  (params (ActionValue :type Boolean) (ElapsedSeconds :type Float%20%28double-precision%29) (TriggeredSeconds :type Float%20%28double-precision%29) (InputAction :type Input%20Action%20Object%20Reference :default "/Game/Core/Blueprints/Input/InputActions/IA_Next.IA_Next"))
  (bind _playeractor (Variables|Default|GetPlayerActor))
  (bind _playerclassname (Variables|Default|GetPlayerClassName))
  ;[1 1 1] Lock character and arena logic
  (:Started
    (if (Utilities|AreBothPlayersReady?)
      (Utilities|FlowControl|Delay 0.2)
      (if ActionValue
        (Default|OpenArenaLogic (Variables|Default|GetGSCharacterSelectionRef)))
      (elif (Utilities|IsServer?)
        (Default|LockCharacter _playeractor _playerclassname)
        (if (Variables|/Game/Core/Blueprints/Characters/CharacterSelector/BP_CharacterSelection.BP_CharacterSelection_C|GetbCanLock? _playeractor)
          (Utilities|FlowControl|FlipFlop
            (:A
              (Variables|Default|SetP1Locked? true)
              (Utilities|FlowControl|Delay 0.01)
              (if (Utilities|AreBothPlayersReady?)
                (Default|OpenArenaSelectionMenu (Variables|Default|GetGSCharacterSelectionRef))))
            (:B
              (Variables|Default|SetP1Locked? false))))
        (else
          (CallFunction|SRLockCharacter _playeractor _playerclassname))))))

(event Input|EnhancedActionEvents|EnhancedInputActionIA_Exit
  (params (ActionValue :type Boolean) (ElapsedSeconds :type Float%20%28double-precision%29) (TriggeredSeconds :type Float%20%28double-precision%29) (InputAction :type Input%20Action%20Object%20Reference :default "/Game/Core/Blueprints/Input/InputActions/IA_Exit.IA_Exit"))
  ;[1 1 1] Server leaving and Client creating new match as Server logic
  (CallFunction|CLLoadingScreen)
  (if (and (Utilities|IsServer?) (Variables|Default|GetbP2))
    (bind _returnvalue (Utilities|Time|SetTimerbyEvent (delegate Custom|LeaveGame) 1.0))
    (bind _asgm_character_selection (Utilities|Casting|CastToGM_CharacterSelection (Game|GetGameMode)))
    (bind _asbpc_character_selection (Utilities|Casting|CastToBPC_CharacterSelection (Utilities|Array|Get(acopy) (Variables|/Game/Core/Blueprints/GameRules/GameModes/GM_CharacterSelection.GM_CharacterSelection_C|GetPlayerControllers _asgm_character_selection) 1)))
    (CallFunction|StartNewServer _asbpc_character_selection)
    (else
      (Game|OpenLevel(byObjectReference) "/Game/maps/L_MainMenu.L_MainMenu"))))

(event EventBeginPlay
  ;[1 1 1] Event BeginPlay
  (Utilities|FlowControl|Sequence
    (:then_0
      (bind _asgi_tiki_tandems (Utilities|Casting|CastToGI_TikiTandems (Game|GetGameInstance)))
      (Variables|Default|SetGIReference _asgi_tiki_tandems)
      (bind _asgs_character_selection (Utilities|Casting|CastToGS_CharacterSelection (Game|GetGameState)))
      (Variables|Default|SetGSCharacterSelectionRef _asgs_character_selection))
    (:then_1
      (CallFunction|CLLoadingScreen)
      (CallFunction|InitializeSelectorData))))

(fn ConstructionScript)

(fn InitializeSelectorData
  (Utilities|FlowControl|Sequence
    (:then_0
      (bind _outactors (Actor|GetAllActorsOfClass "/Game/Core/Blueprints/Characters/CharacterSelector/BP_CharacterSelection.BP_CharacterSelection_C"))
      (for (_array_element _array_index) _outactors
        (switch int _array_index
          (:0
            (Variables|Default|SetP1Actor _array_element))
          (:1
            (Variables|Default|SetP2Actor _array_element)))))
    (:then_1
      (bind _outactors_2 (Actor|GetAllActorsOfClass "/Game/Core/Widgets/MainMenu/W_WorldButton.W_WorldButton_C"))
      (for (_array_element_2 _array_index_2) _outactors_2
        (switch int _array_index_2
          (:0
            (Variables|Default|SetP1ClassName _array_element_2))
          (:1
            (Variables|Default|SetP2ClassName _array_element_2)))))))

(fn SwitchCharacter
  (params (NextPrev :type Boolean) (WhichPlayer? :type BP%20Character%20Selection%20Object%20Reference))
  (if NextPrev
    (bind _selectedcharacter (CallFunction|NextCharacter WhichPlayer?))
    (Variables|Default|SeteSelectedCharacter _selectedcharacter)
    (else
      (bind _selectedcharacter_2 (CallFunction|PreviousCharacter WhichPlayer?))
      (Variables|Default|SeteSelectedCharacter _selectedcharacter_2))))

(fn NextCharacter
  (params (Swticher :type BP%20Character%20Selection%20Object%20Reference))
  (Default|FlipAnimation Swticher true)
  (switch Utilities|FlowControl|Switch|SwitchonE_CharacterClasses (Variables|/Game/Core/Blueprints/Characters/CharacterSelector/BP_CharacterSelection.BP_CharacterSelection_C|GeteCurrentCharacter Swticher)
    (:NewEnumerator0
      (bind _output_get (Variables|/Game/Core/Blueprints/Characters/CharacterSelector/BP_CharacterSelection.BP_CharacterSelection_C|SeteCurrentCharacter Swticher "NewEnumerator1"))
      (return _output_get))
    (:NewEnumerator1
      (bind _output_get_2 (Variables|/Game/Core/Blueprints/Characters/CharacterSelector/BP_CharacterSelection.BP_CharacterSelection_C|SeteCurrentCharacter Swticher "NewEnumerator2"))
      (return _output_get_2))
    (:NewEnumerator2
      (bind _output_get_3 (Variables|/Game/Core/Blueprints/Characters/CharacterSelector/BP_CharacterSelection.BP_CharacterSelection_C|SeteCurrentCharacter Swticher "NewEnumerator0"))
      (return _output_get_3))))

(fn PreviousCharacter
  (params (Switcher :type BP%20Character%20Selection%20Object%20Reference))
  (Default|FlipAnimation Switcher false)
  (switch Utilities|FlowControl|Switch|SwitchonE_CharacterClasses (Variables|/Game/Core/Blueprints/Characters/CharacterSelector/BP_CharacterSelection.BP_CharacterSelection_C|GeteCurrentCharacter Switcher)
    (:NewEnumerator0
      (bind _output_get (Variables|/Game/Core/Blueprints/Characters/CharacterSelector/BP_CharacterSelection.BP_CharacterSelection_C|SeteCurrentCharacter Switcher "NewEnumerator2"))
      (return _output_get))
    (:NewEnumerator1
      (bind _output_get_2 (Variables|/Game/Core/Blueprints/Characters/CharacterSelector/BP_CharacterSelection.BP_CharacterSelection_C|SeteCurrentCharacter Switcher "NewEnumerator0"))
      (return _output_get_2))
    (:NewEnumerator2
      (bind _output_get_3 (Variables|/Game/Core/Blueprints/Characters/CharacterSelector/BP_CharacterSelection.BP_CharacterSelection_C|SeteCurrentCharacter Switcher "NewEnumerator1"))
      (return _output_get_3))))

(fn GetPlayerCharacterClass
  (params (CharacterSelection :type E_CharacterClasses%20Enum :default "NewEnumerator0"))
  (switch Utilities|FlowControl|Switch|SwitchonE_CharacterClasses CharacterSelection
    (:NewEnumerator0
      (return "/Game/Core/Blueprints/Characters/Spearman/BP_Spearman.BP_Spearman_C"))
    (:NewEnumerator1
      (return "/Game/Core/Blueprints/Characters/Bonkerman/BP_Bonkerman.BP_Bonkerman_C"))
    (:NewEnumerator2
      (return "/Game/Core/Blueprints/Characters/Magicman/BP_Magicman.BP_Magicman_C"))))

(fn OnRepP1Locked?
  (bind _self self)
  (if (Variables|Default|GetP1Locked?)
    (CallFunction|RemoveInputMappingContext _self "/Game/Core/Blueprints/Input/InputActionMappings/IMC_CharacterSelection.IMC_CharacterSelection")
    (CallFunction|AddInputMappingContext _self "/Game/Core/Blueprints/Input/InputActionMappings/IMC_Lock.IMC_Lock" 1)
    (else
      (CallFunction|RemoveInputMappingContext _self "/Game/Core/Blueprints/Input/InputActionMappings/IMC_Lock.IMC_Lock")
      (CallFunction|AddInputMappingContext _self "/Game/Core/Blueprints/Input/InputActionMappings/IMC_CharacterSelection.IMC_CharacterSelection" 1))))

(fn OnRepP2Locked?
  (bind _self self)
  (bind _p2classname (Variables|Default|GetP2ClassName))
  (if (Variables|Default|GetP2Locked?)
    (CallFunction|RemoveInputMappingContext _self "/Game/Core/Blueprints/Input/InputActionMappings/IMC_CharacterSelection.IMC_CharacterSelection")
    (CallFunction|AddInputMappingContext _self "/Game/Core/Blueprints/Input/InputActionMappings/IMC_Lock.IMC_Lock" 1)
    (Default|UpdateTextColor _p2classname)
    (else
      (CallFunction|RemoveInputMappingContext _self "/Game/Core/Blueprints/Input/InputActionMappings/IMC_Lock.IMC_Lock")
      (CallFunction|AddInputMappingContext _self "/Game/Core/Blueprints/Input/InputActionMappings/IMC_CharacterSelection.IMC_CharacterSelection" 1)
      (Default|UpdateTextColor _p2classname "(R=1.000000,G=1.000000,B=1.000000,A=1.000000)"))))

(fn OnRepESelectedCharacter
  (CallFunction|CLSetPlayerClass))

(fn SetSelectedPlayer
  (params (PlayerIndex :type Integer))
  (bind _output_get (Variables|Default|SetiPlayerIndex PlayerIndex))
  (switch int _output_get
    (:0
      (Variables|Default|SetPlayerActor (Variables|Default|GetP1Actor))
      (Variables|Default|SetPlayerClassName (Variables|Default|GetP1ClassName)))
    (:1
      (Variables|Default|SetPlayerActor (Variables|Default|GetP2Actor))
      (Variables|Default|SetPlayerClassName (Variables|Default|GetP2ClassName)))))