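; Player controller for the Tiki arena mode that spawns the player's character and handles input, loading screen and pause menu.
; BeginPlay shows the loading widget and has GM_Arena spawn the game instance's class for this player index, with Red/Blue teams by index parity.
; After a short delay it caches the BP_Tiki pawn and creates its overlay.
; Enhanced Input forwards to that pawn, while pausing swaps combat and exit mapping contexts.
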(event Custom|SR_Spawn
  (params (Class :type BP%20Tiki%20Class%20Reference) (TeamTag :type Name))
  ;[1 1 1] Begin play
  (bind _asgm_arena (Utilities|Casting|CastToGM_Arena (Game|GetGameMode)))
  (Default|SpawnandPossessPlayer _asgm_arena self Class TeamTag))

(event Custom|AddControls
  ;[1 1 1] Add controls and UI
  (CallFunction|AddInputMappingContext self "/Game/Core/Blueprints/Input/InputActionMappings/IMC_Combat.IMC_Combat" 1))

(event Custom|PauseGame
  (bind _self self)
  ;[1 1 1] Pause/Resume game logic
  (bind _returnvalue (UserInterface|CreateWidget "/Game/Core/Widgets/NewWidgets/W_PauseMenu.W_PauseMenu_C" _self))
  (bind _output_get (Variables|Default|SetwPauseMenu _returnvalue))
  (UserInterface|Viewport|AddtoViewport _output_get 0)
  (Input|SetInputModeGameandUI _self 0 "DoNotLock" true false)
  (Variables|Default|SetbShowMouseCursor _self true)
  (CallFunction|AddInputMappingContext _self "/Game/Core/Blueprints/Input/InputActionMappings/IMC_Exit.IMC_Exit" 1)
  (CallFunction|RemoveInputMappingContext _self "/Game/Core/Blueprints/Input/InputActionMappings/IMC_Combat.IMC_Combat"))

(event Custom|ResumeGame
  (bind _self self)
  ;[1 1 1] Pause/Resume game logic
  (Widget|RemovefromParent (Variables|Default|GetwPauseMenu))
  (Input|SetInputModeGameOnly _self false)
  (Variables|Default|SetbShowMouseCursor _self false)
  (Class|WidgetBlueprintLibrary|SetFocustoGameViewport)
  (CallFunction|AddInputMappingContext _self "/Game/Core/Blueprints/Input/InputActionMappings/IMC_Combat.IMC_Combat" 1)
  (CallFunction|RemoveInputMappingContext _self "/Game/Core/Blueprints/Input/InputActionMappings/IMC_Exit.IMC_Exit"))

(event Custom|CL_CreateLoadingScreen
  ;[1 1 1] LoadingWidget logic
  (bind _returnvalue (UserInterface|CreateWidget "/Game/Core/Widgets/MainMenu/W_TransitionWidget.W_TransitionWidget_C" self))
  (bind _output_get (Variables|Default|SetwLoading _returnvalue))
  (UserInterface|Viewport|AddtoViewport _output_get 3))

(event Custom|CL_RemoveLoadingScreen
  ;[1 1 1] LoadingWidget logic
  (Widget|RemovefromParent (Variables|Default|GetwLoading)))

(event Input|EnhancedActionEvents|EnhancedInputActionIA_Look
  (params (ActionValue :type Vector%202D%20Structure) (ElapsedSeconds :type Float%20%28double-precision%29) (TriggeredSeconds :type Float%20%28double-precision%29) (InputAction :type Input%20Action%20Object%20Reference :default "/Game/Core/Blueprints/Input/InputActions/IA_Look.IA_Look"))
  ;[1 1 1] Basic input
  (Default|LookInput (Variables|Default|GetBPTikiReference) (.x ActionValue) (.y ActionValue)))

(event Input|EnhancedActionEvents|EnhancedInputActionIA_Move
  (params (ActionValue :type Vector%202D%20Structure) (ElapsedSeconds :type Float%20%28double-precision%29) (TriggeredSeconds :type Float%20%28double-precision%29) (InputAction :type Input%20Action%20Object%20Reference :default "/Game/Core/Blueprints/Input/InputActions/IA_Move.IA_Move"))
  ;[1 1 1] Basic input
  (Default|MoveInput (Variables|Default|GetBPTikiReference) (.x ActionValue) (.y ActionValue)))

(event Input|EnhancedActionEvents|EnhancedInputActionIA_Jump
  (params (ActionValue :type Boolean) (ElapsedSeconds :type Float%20%28double-precision%29) (TriggeredSeconds :type Float%20%28double-precision%29) (InputAction :type Input%20Action%20Object%20Reference :default "/Game/Core/Blueprints/Input/InputActions/IA_Jump.IA_Jump"))
  ;[1 1 1] Basic input
  (:Started
    (Default|JumpInput (Variables|Default|GetBPTikiReference))))

(event Input|EnhancedActionEvents|EnhancedInputActionIA_BasicAttack
  (params (ActionValue :type Boolean) (ElapsedSeconds :type Float%20%28double-precision%29) (TriggeredSeconds :type Float%20%28double-precision%29) (InputAction :type Input%20Action%20Object%20Reference :default "/Game/Core/Blueprints/Input/InputActions/IA_BasicAttack.IA_BasicAttack"))
  (bind _bptikireference (Variables|Default|GetBPTikiReference))
  ;[1 1 1] Combat input
  (:Triggered
    (Class|BPICombat|ICBasicAttackTriggered(Message) _bptikireference ElapsedSeconds))
  (:Started
    (Class|BPICombat|ICBasicAttackStarted(Message) _bptikireference))
  (:Completed
    (Class|BPICombat|ICBasicAttackCompleted(Message) _bptikireference)))

(event Input|EnhancedActionEvents|EnhancedInputActionIA_SpecialAttack
  (params (ActionValue :type Boolean) (ElapsedSeconds :type Float%20%28double-precision%29) (TriggeredSeconds :type Float%20%28double-precision%29) (InputAction :type Input%20Action%20Object%20Reference :default "/Game/Core/Blueprints/Input/InputActions/IA_SpecialAttack.IA_SpecialAttack"))
  ;[1 1 1] Combat input
  (:Started
    (Class|BPICombat|ICSpecialAttackStarted(Message) (Variables|Default|GetBPTikiReference))))

(event Input|EnhancedActionEvents|EnhancedInputActionIA_HeavyAttack
  (params (ActionValue :type Boolean) (ElapsedSeconds :type Float%20%28double-precision%29) (TriggeredSeconds :type Float%20%28double-precision%29) (InputAction :type Input%20Action%20Object%20Reference :default "/Game/Core/Blueprints/Input/InputActions/IA_HeavyAttack.IA_HeavyAttack"))
  ;[1 1 1] Combat input
  (:Started
    (Class|BPICombat|ICHeavyAttackStarted(Message) (Variables|Default|GetBPTikiReference))))

(event Input|EnhancedActionEvents|EnhancedInputActionIA_Exit
  (params (ActionValue :type Boolean) (ElapsedSeconds :type Float%20%28double-precision%29) (TriggeredSeconds :type Float%20%28double-precision%29) (InputAction :type Input%20Action%20Object%20Reference :default "/Game/Core/Blueprints/Input/InputActions/IA_Exit.IA_Exit"))
  ;[1 1 1] Combat input
  (:Started
    (Utilities|FlowControl|FlipFlop
      (:A
        (CallFunction|PauseGame))
      (:B
        (CallFunction|ResumeGame)))))

(event EventBeginPlay
  ;[1 1 1] Begin play
  (CallFunction|CLCreateLoadingScreen)
  (CallFunction|SpawnCharacter)
  (Utilities|FlowControl|Delay 0.2)
  (bind _asbp_tiki (Utilities|Casting|CastToBP_Tiki (Pawn|GetControlledPawn)))
  (bind _output_get (Variables|Default|SetBPTikiReference _asbp_tiki))
  (Default|CreateGameOverlay _output_get)
  (Input|SetInputModeGameOnly self false))

(fn ConstructionScript)

(fn SpawnCharacter
  (bind _iplayerindex (Variables|Default|GetiPlayerIndex))
  (bind _asgi_tiki_tandems (Utilities|Casting|CastToGI_TikiTandems (Game|GetGameInstance)))
  (if (== (Math|Integer|%(Integer) _iplayerindex 2) 0)
    (CallFunction|SRSpawn (Utilities|Array|Get(acopy) (Variables|/Game/Core/Blueprints/GameRules/GI_TikiTandems.GI_TikiTandems_C|GetPlayerClasses _asgi_tiki_tandems) _iplayerindex) "Red")
    (else
      (CallFunction|SRSpawn (Utilities|Array|Get(acopy) (Variables|/Game/Core/Blueprints/GameRules/GI_TikiTandems.GI_TikiTandems_C|GetPlayerClasses _asgi_tiki_tandems) _iplayerindex) "Blue"))))