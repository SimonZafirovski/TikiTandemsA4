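; Player controller for the end screen that shows the win widget three seconds after BeginPlay and gives its Quick button focus on gamepad input.
; Quick game searches EIK matchmaking sessions named "Public" and joins a random result.
; If search or join fails, it creates a two-player session and server-travels to online character selection as a listen server.
; Quitting destroys the session, then opens the main menu after a delay.
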(event Custom|NewQuickGame
  (bind _sessionresults (|FindEIKSessions (Utilities|Map|MakeMap "SessionName" (Utilities|Struct|MakeEIKAttribute "String" "Public" false)) "MT_MatchMakingSession" 50 "RE_NoSelection")
    (:OnSuccess
      (|JoinEIKSessions (.OutItem (Utilities|Array|Random _sessionresults))
        (:OnFail
          _)))
    (:OnFail
      _))
  (|EIKSession (Utilities|Map|MakeMap "SessionName" (Utilities|Struct|MakeEIKAttribute "String" "Public" false)) 2 "(bIsDedicatedServer=False,PortInfo=0)" (Utilities|Struct|MakeCreateSessionExtraSettings 0 true)
    (:OnSuccess
      (Development|ExecuteConsoleCommand (Utilities|String|Append "servertravel " "L_CharacterSelectionOnline" "?listen") 0))))

(event Custom|QuitGame
  (|DestroyEIKSessions
    (:then
      (Utilities|FlowControl|Delay 2.0)
      (Game|OpenLevel(byObjectReference) "/Game/maps/L_MainMenu.L_MainMenu"))))

(event EventBeginPlay
  (Utilities|FlowControl|Delay 3.0)
  (bind _returnvalue (UserInterface|CreateWidget "/Game/Core/Widgets/MainMenu/W_WinScreen.W_WinScreen_C"))
  (bind _output_get (Variables|Default|SetwWinScreen _returnvalue))
  (UserInterface|Viewport|AddtoViewport _output_get 0))

(event Input|KeyboardEvents|AnyKey
  (params (Key :type Key%20Structure :default "None"))
  (bind _wwinscreen (Variables|Default|GetwWinScreen))
  (:Pressed
    (if (Class|KismetInputLibrary|KeyIsGamepadKey Key)
      (Utilities|IsValid _wwinscreen
        (:Is%20Valid
          (Widget|SetFocus (Variables|/Game/Core/Widgets/MainMenu/W_WinScreen.W_WinScreen_C|GetQuick _wwinscreen))))
      (else
        (Class|WidgetBlueprintLibrary|SetFocustoGameViewport)))))

(fn ConstructionScript)