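; End-screen character that displays the match winner or loser, chosen by a "Winner" actor tag; losers get a separate anim class at construction.
; On BeginPlay it reads the game instance, identifies spearman, bonkerman or magicman by class-name substring, and sets a team-colour overlay from player index parity and arena type.
; It plays a delayed win or lose montage, then a looping timer triggers further montages after random delays.
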(event Custom|SetCharacter
  (bind _asgi_tiki_tandems (Utilities|Casting|CastToGI_TikiTandems (Game|GetGameInstance)))
  (if (Actor|ActorHasTag "Winner")
    (Utilities|SwitchonBPTikiClass (Variables|/Game/Core/Blueprints/GameRules/GI_TikiTandems.GI_TikiTandems_C|GetWinner _asgi_tiki_tandems))
    (CallFunction|SetTeamColor (Variables|/Game/Core/Blueprints/GameRules/GI_TikiTandems.GI_TikiTandems_C|GetWinnerIndex _asgi_tiki_tandems))
    (else
      (Utilities|SwitchonBPTikiClass (Variables|/Game/Core/Blueprints/GameRules/GI_TikiTandems.GI_TikiTandems_C|GetLoser _asgi_tiki_tandems))
      (CallFunction|SetTeamColor (Variables|/Game/Core/Blueprints/GameRules/GI_TikiTandems.GI_TikiTandems_C|GetLoserIndex _asgi_tiki_tandems))))
  (switch Utilities|FlowControl|Switch|SwitchonE_CharacterClasses (Variables|Default|GeteCurrentCharacter)
    (:NewEnumerator0
      (Utilities|PlayAnimations true "/Game/Assets/TikiCharacter/Animations/Spearman/AM_LockSpearman.AM_LockSpearman" "/Game/Assets/TikiCharacter/Animations/Shared/AM_LoseAnim.AM_LoseAnim")
      (Utilities|Time|SetTimerbyEvent (delegate Custom|LoopSpearman) 5.0 true))
    (:NewEnumerator1
      (Utilities|PlayAnimations true "/Game/Assets/TikiCharacter/Animations/Bonkerman/AM_BonkermanWin.AM_BonkermanWin" "/Game/Assets/TikiCharacter/Animations/Shared/AM_LoseAnim.AM_LoseAnim")
      (Utilities|Time|SetTimerbyEvent (delegate Custom|LoopBonkerman) 5.0 true))
    (:NewEnumerator2
      (Utilities|PlayAnimations true "/Game/Assets/TikiCharacter/Animations/Magicman/AM_Magicman_Win.AM_Magicman_Win" "/Game/Assets/TikiCharacter/Animations/Shared/AM_LoseAnim.AM_LoseAnim")
      (Utilities|Time|SetTimerbyEvent (delegate Custom|LoopMagicman) 5.0 true))))

(event Custom|LoopMagicman
  (Utilities|PlayAnimations false "/Game/Assets/TikiCharacter/Animations/Magicman/AM_LockMagicMan.AM_LockMagicMan" "/Game/Assets/TikiCharacter/Animations/Shared/AM_Cry.AM_Cry"))

(event Custom|LoopSpearman
  (Utilities|PlayAnimations false "/Game/Assets/TikiCharacter/Animations/Spearman/AM_LockSpearman.AM_LockSpearman" "/Game/Assets/TikiCharacter/Animations/Shared/AM_Cry.AM_Cry"))

(event Custom|LoopBonkerman
  (Utilities|PlayAnimations false "/Game/Assets/TikiCharacter/Animations/Bonkerman/AM_LockBonkerman.AM_LockBonkerman" "/Game/Assets/TikiCharacter/Animations/Shared/AM_Cry.AM_Cry"))

(event EventBeginPlay
  (|CallParentFunction)
  (CallFunction|SetCharacter))

(fn ConstructionScript
  (if (not (Actor|ActorHasTag "Winner"))
    (Class|SkeletalMeshComponent|SetAnimClass (Variables|Character|GetMesh) "/Game/Assets/TikiCharacter/Animations/Shared/ABP_WildmanLose.ABP_WildmanLose_C")))

(fn SetTeamColor
  (params (PlayerIndex :type Integer))
  (bind _returnvalue (Math|Integer|%(Integer) PlayerIndex 2))
  (bind _mesh (Variables|Character|GetMesh))
  (bind _returnvalue_2 (== _returnvalue 0))
  (bind _asgi_tiki_tandems (Utilities|Casting|CastToGI_TikiTandems (Game|GetGameInstance)))
  (switch Utilities|FlowControl|Switch|SwitchonE_ArenaType (Variables|/Game/Core/Blueprints/GameRules/GI_TikiTandems.GI_TikiTandems_C|GeteArenaType _asgi_tiki_tandems)
    (:NewEnumerator0
      (if _returnvalue_2
        (Rendering|Material|SetOverlayMaterial _mesh "/Game/Assets/TikiCharacter/Materials/MI_RedPlayer.MI_RedPlayer" :!class /Script/Engine.MeshComponent)
        (else
          (Rendering|Material|SetOverlayMaterial _mesh "/Game/Assets/TikiCharacter/Materials/MI_BluePlayer.MI_BluePlayer" :!class /Script/Engine.MeshComponent))))
    (:NewEnumerator1
      (if _returnvalue_2
        (Rendering|Material|SetOverlayMaterial _mesh "/Game/Assets/TikiCharacter/Materials/MI_PurplePLayer.MI_PurplePLayer" :!class /Script/Engine.MeshComponent)
        (else
          (Rendering|Material|SetOverlayMaterial _mesh "/Game/Assets/TikiCharacter/Materials/MI_YellowPlayer.MI_YellowPlayer" :!class /Script/Engine.MeshComponent))))))